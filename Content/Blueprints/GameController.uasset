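; GameController is a game manager Blueprint that spawns enemies around the player and accumulates score.
; On BeginPlay, if an enemy class is set, a looping timer calls SpawnEnemy at the configured per-second rate.
; Each spawn lands at a fixed X distance randomly either side of the PlayerBP pawn, on the Y=0 plane, with randomly flipped rotation.
; AddScore adds incoming points to TargetScore.
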(event Custom|AddScore
  (params (AddScorePoints :type Integer))
  (Variables|Default|SetTargetScore (+ AddScorePoints (Variables|Default|GetTargetScore))))

(event Custom|SpawnEnemy
  (bind _returnvalue (Game|Player|GetPlayerPawn 0))
  (bind _returnvalue_2 (Math|Random|RandomBool))
  (bind _returnvalue_3 (Transformation|GetActorLocation _returnvalue))
  (bind (_x _y _z) (Math|Vector|BreakVector _returnvalue_3))
  (Utilities|Casting|CastToPlayerBP (Game|Player|GetPlayerPawn 0))
  (Utilities|IsValid _returnvalue
    (:Is%20Valid
      (Game|SpawnActorfromClass (Variables|Default|GetEnemyClass) (Math|Transform|MakeTransform (Math|Vector|MakeVector (+ _x (* (Math|Integer|SelectInt 1 -1 _returnvalue_2) 1.2e+03)) 0.0 (+ _z (Math|Random|RandomFloatinRange 5.0 5.0))) (Math|Rotator|SelectRotator "0,180.000000, 0" "0, 0,0.000000" _returnvalue_2)) "AdjustIfPossibleButDontSpawnIfColliding" 0 0))))

(event EventBeginPlay
  (Utilities|FlowControl|Sequence
    (:then_1
      (if (!= (Variables|Default|GetEnemyClass) 0)
        (Utilities|Time|SetTimerbyFunctionName 0 "SpawnEnemy" (/ 1.0 (Variables|Default|GetEnemiesPerSecond)) true)))))

(fn ConstructionScript)