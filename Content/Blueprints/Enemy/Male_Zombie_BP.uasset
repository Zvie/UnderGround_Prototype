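; Male zombie enemy for a flipbook-based game, damaging the player on overlap and awarding score on death.
; EnemyTimeline is set up to ping-pong it between StartPoint and EndPoint, with play rate derived from MovementRate.
; Tick picks attack or walk flipbooks from Sight overlap; death halts the timeline and delays destruction.
; The construction script can preview EndPoint and snap the actor to Y=0 via TestEndPoint.
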(event OnComponentBeginOverlap(sight)
  (params (OverlappedComponent :type Primitive%20Component%20Object%20Reference) (OtherActor :type Actor%20Object%20Reference) (OtherComp :type Primitive%20Component%20Object%20Reference) (OtherBodyIndex :type Integer) (bFromSweep :type Boolean) (SweepResult :type Hit%20Result%20Structure%20%28by%20ref%29))
  ;[1 1 1] Player overlap
  (Variables|Default|SetinRange true))

(event OnComponentEndOverlap(sight)
  (params (OverlappedComponent :type Primitive%20Component%20Object%20Reference) (OtherActor :type Actor%20Object%20Reference) (OtherComp :type Primitive%20Component%20Object%20Reference) (OtherBodyIndex :type Integer))
  ;[1 1 1] Player overlap
  (Variables|Default|SetinRange false))

(event OnComponentBeginOverlap(enemy)
  (params (OverlappedComponent :type Primitive%20Component%20Object%20Reference) (OtherActor :type Actor%20Object%20Reference) (OtherComp :type Primitive%20Component%20Object%20Reference) (OtherBodyIndex :type Integer) (bFromSweep :type Boolean) (SweepResult :type Hit%20Result%20Structure%20%28by%20ref%29))
  ;[1 1 1] Hit Player
  (bind _asplayer_bp (Utilities|Casting|CastToPlayerBP OtherActor))
  (Default|Damage _asplayer_bp (Variables|Default|GetDmgAmt_M_Zombie)))

(event Custom|DamageEnemy
  (params (damage :type Float%20%28single-precision%29))
  ;[1 1 1] Damage
  (bind _output_get (Variables|Default|SetHealth (- (Variables|Default|GetHealth) damage)))
  (if (<= _output_get 0.0)
    (Components|Timeline|SetPlayRate (Variables|Default|GetEnemyTimeline) 0.0)
    (bind _returnvalue (AddComponent|AddAudioComponent false))
    (Sprite|SetFlipbook (Variables|Default|Getenemy) "/Game/Flipbooks/Enemy/Zombie_M/M_Zombie_Death_FB.M_Zombie_Death_FB")
    (bind _asgame_controller (Utilities|Casting|CastToGameController (Game|GetGameMode)))
    (Default|AddScore _asgame_controller (Variables|Default|Getscoreadd))
    (Utilities|FlowControl|Delay 0.7)
    (Audio|Components|Audio|Stop _returnvalue)
    (Actor|DestroyActor)))

(event EventBeginPlay
  ;[1 1 1] Movement
  (Components|Timeline|SetPlayRate (Variables|Default|GetEnemyTimeline) (/ 1.0 (Variables|Default|GetMovementRate))))

(event EventTick
  (params (DeltaSeconds :type Float%20%28single-precision%29))
  ;[1 1 1] Male Zombie Melee
  (if (> (Variables|Default|GetHealth) 0.0)
    (if (Variables|Default|GetinRange)
      (Sprite|SetFlipbook (Variables|Default|Getenemy) "/Game/Flipbooks/Enemy/Zombie_M/M_Zombie_Attack_FB.M_Zombie_Attack_FB")
      (else
        (Sprite|SetFlipbook (Variables|Default|Getenemy) "/Game/Flipbooks/Enemy/Zombie_M/M_Zombie_Walk_FB.M_Zombie_Walk_FB")))))

(fn ConstructionScript
  (bind _returnvalue (Transformation|GetActorLocation))
  (bind (_x _y _z) (Math|Vector|BreakVector _returnvalue))
  (if (Variables|Default|GetTestEndPoint%20)
    (Transformation|SetRelativeLocation (Variables|Default|Getenemy) (Variables|Default|GetEndPoint) false false)
    (Transformation|SetActorLocation (Math|Vector|MakeVector _x 0.0 _z) false false)))