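; Paper2D boss enemy that fires projectile volleys, hurts the player on contact, and opens the win level when killed.
; EnemyTimeline is set up to ping-pong the flipbook between two points, flipping it at each end, though nothing here starts it.
; While the Sight overlap holds, a Delay on Tick paces nine-arrow volleys; Tick also updates the health bar widget.
; Death freezes movement, swaps the flipbook and awards score before destroying the actor.
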(event OnComponentBeginOverlap(sight)
  (params (OverlappedComponent :type Primitive%20Component%20Object%20Reference) (OtherActor :type Actor%20Object%20Reference) (OtherComp :type Primitive%20Component%20Object%20Reference) (OtherBodyIndex :type Integer) (bFromSweep :type Boolean) (SweepResult :type Hit%20Result%20Structure%20%28by%20ref%29))
  ;[1 1 1] Player overlap
  (Variables|Default|SetinRange true))

(event OnComponentEndOverlap(sight)
  (params (OverlappedComponent :type Primitive%20Component%20Object%20Reference) (OtherActor :type Actor%20Object%20Reference) (OtherComp :type Primitive%20Component%20Object%20Reference) (OtherBodyIndex :type Integer))
  ;[1 1 1] Player overlap
  (Variables|Default|SetinRange false))

(event OnComponentBeginOverlap(enemy)
  (params (OverlappedComponent :type Primitive%20Component%20Object%20Reference) (OtherActor :type Actor%20Object%20Reference) (OtherComp :type Primitive%20Component%20Object%20Reference) (OtherBodyIndex :type Integer) (bFromSweep :type Boolean) (SweepResult :type Hit%20Result%20Structure%20%28by%20ref%29))
  ;[1 1 1] Hit Player
  (bind _asplayer_bp (Utilities|Casting|CastToPlayerBP OtherActor))
  (Default|Damage _asplayer_bp (Variables|Default|GetDmgAmt)))

(event Custom|DamageEnemy
  (params (damage :type Float%20%28single-precision%29))
  ;[1 1 1] Damage
  (bind _output_get (Variables|Default|SetHealth (- (Variables|Default|GetHealth) damage)))
  (if (<= _output_get 0.0)
    (Components|Timeline|SetPlayRate (Variables|Default|GetEnemyTimeline) 0.0)
    (Sprite|SetFlipbook (Variables|Default|Getenemy) "/Game/Flipbooks/Enemy/Boss/Boss_Ded_FB.Boss_Ded_FB")
    (bind _asgame_controller (Utilities|Casting|CastToGameController (Game|GetGameMode)))
    (Default|AddScore _asgame_controller (Variables|Default|GetTargetScore))
    (Utilities|FlowControl|Delay 1.0)
    (Actor|DestroyActor)
    (Game|OpenLevel(byName) "GameOver_Win")))

(event EventTick
  (params (DeltaSeconds :type Float%20%28single-precision%29))
  (bind _projectilearrow_7 (Variables|Default|GetProjectileArrow_7))
  (bind _projectilearrow_9 (Variables|Default|GetProjectileArrow_9))
  (bind _projectilearrow_2 (Variables|Default|GetProjectileArrow_2))
  (bind _projectilearrow_8 (Variables|Default|GetProjectileArrow_8))
  (bind _projectilearrow_3 (Variables|Default|GetProjectileArrow_3))
  (bind _projectilearrow_4 (Variables|Default|GetProjectileArrow_4))
  (bind _projectilearrow_5 (Variables|Default|GetProjectileArrow_5))
  (bind _projectilearrow_6 (Variables|Default|GetProjectileArrow_6))
  (Utilities|FlowControl|Sequence
    (:then_0
      ;[1 1 1] firing
      (if (> (Variables|Default|GetHealth) 0.0)
        (if (Variables|Default|GetinRange)
          (Utilities|FlowControl|Delay 1.0)
          (Game|SpawnActorfromClass "/Game/Blueprints/Enemy/EnemyProjectile.EnemyProjectile_C" (Math|Transform|MakeTransform (Transformation|GetWorldLocation (Variables|Default|GetprojectileArrow)) (Transformation|GetWorldRotation (Variables|Default|GetprojectileArrow))) "Undefined" 0 0)
          (Game|SpawnActorfromClass "/Game/Blueprints/Enemy/EnemyProjectile.EnemyProjectile_C" (Math|Transform|MakeTransform (Transformation|GetWorldLocation _projectilearrow_2) (Transformation|GetWorldRotation _projectilearrow_2)) "Undefined" 0 0)
          (Game|SpawnActorfromClass "/Game/Blueprints/Enemy/EnemyProjectile.EnemyProjectile_C" (Math|Transform|MakeTransform (Transformation|GetWorldLocation _projectilearrow_3) (Transformation|GetWorldRotation _projectilearrow_3)) "Undefined" 0 0)
          (Game|SpawnActorfromClass "/Game/Blueprints/Enemy/EnemyProjectile.EnemyProjectile_C" (Math|Transform|MakeTransform (Transformation|GetWorldLocation _projectilearrow_4) (Transformation|GetWorldRotation _projectilearrow_4)) "Undefined" 0 0)
          (Game|SpawnActorfromClass "/Game/Blueprints/Enemy/EnemyProjectile.EnemyProjectile_C" (Math|Transform|MakeTransform (Transformation|GetWorldLocation _projectilearrow_5) (Transformation|GetWorldRotation _projectilearrow_5)) "Undefined" 0 0)
          (Game|SpawnActorfromClass "/Game/Blueprints/Enemy/EnemyProjectile.EnemyProjectile_C" (Math|Transform|MakeTransform (Transformation|GetWorldLocation _projectilearrow_6) (Transformation|GetWorldRotation _projectilearrow_6)) "Undefined" 0 0)
          (Game|SpawnActorfromClass "/Game/Blueprints/Enemy/EnemyProjectile.EnemyProjectile_C" (Math|Transform|MakeTransform (Transformation|GetWorldLocation _projectilearrow_7) (Transformation|GetWorldRotation _projectilearrow_7)) "Undefined" 0 0)
          (Game|SpawnActorfromClass "/Game/Blueprints/Enemy/EnemyProjectile.EnemyProjectile_C" (Math|Transform|MakeTransform (Transformation|GetWorldLocation _projectilearrow_8) (Transformation|GetWorldRotation _projectilearrow_8)) "Undefined" 0 0)
          (Game|SpawnActorfromClass "/Game/Blueprints/Enemy/EnemyProjectile.EnemyProjectile_C" (Math|Transform|MakeTransform (Transformation|GetWorldLocation _projectilearrow_9) (Transformation|GetWorldRotation _projectilearrow_9)) "Undefined" 0 0)
          (Audio|PlaySound2D "/Game/Sound/FX/Snd_Cue/Boss_Projectile_Cue.Boss_Projectile_Cue"))))
    (:then_1
      (bind _asboss_health (Utilities|Casting|CastToBoss_Health (UserInterface|GetUserWidgetObject (Variables|Default|GetWidget))))
      (Progress|SetPercent (Variables|/Game/Widgets/Boss_Health.Boss_Health_C|GetBoss_Health _asboss_health) (/ (Variables|Default|GetHealth) (Variables|Default|GetMaxHealth))))))

(event EventBeginPlay
  ;[1 1 1] Movement
  (Components|Timeline|SetPlayRate (Variables|Default|GetEnemyTimeline) (/ 1.0 (Variables|Default|GetMovementRate))))

(fn ConstructionScript
  (bind _returnvalue (Transformation|GetActorLocation))
  (bind (_x _y _z) (Math|Vector|BreakVector _returnvalue))
  (if (Variables|Default|GetTestEndPoint%20)
    (Transformation|SetRelativeLocation (Variables|Default|Getenemy) (Variables|Default|GetEndPoint) false false)
    (Transformation|SetActorLocation (Math|Vector|MakeVector _x 0.0 _z) false false)))