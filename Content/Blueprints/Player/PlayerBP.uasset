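; Player character for a 2D flipbook side-scroller, handling movement, jumping, trace-based wall jumps, ammo-limited shooting and level doors.
; Movement, firing and damage update state flags that a priority-ordered function maps to sprite flipbooks.
; Damage applies knockback with brief invulnerability; death either loads game over or destroys the actor, whose Destroyed event spawns and possesses a replacement at its construction transform.
; GameInstance carries health, spawn location and level between maps.
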(event Custom|UpdateAnimation
  ;[1 1 1] Animation
  (Variables|Default|SetisMoving (Class|LowEntryExtendedStandardLibrary|GreaterFloatByte (Math|Vector|VectorLength (Transformation|GetVelocity))))
  (Variables|Default|SetisFalling (AI|Components|NavMovement|IsFalling (Variables|Character|GetCharacterMovement)))
  (bind _outputflipbook (CallFunction|AnimationStateMachine (Variables|Default|GetisMoving) (Variables|Default|GetisFalling) (Variables|Default|GetisFiring) (Variables|Default|GetisHurt) (Variables|Default|GetisDead) (Variables|Default|GetisFireMovement)))
  (Sprite|SetFlipbook (Variables|Default|GetSprite) _outputflipbook))

(event Custom|Wall%20Jump
  (bind _returnvalue (Transformation|GetActorForwardVector))
  ;[1 1 1] wall Jump
  (bind (_outhit _returnvalue_2) (Collision|LineTraceByChannel (- (Transformation|GetActorLocation) (* _returnvalue (+ (Components|Capsule|GetScaledCapsuleRadius (Variables|Collision|GetCapsuleComponent)) 15.0))) (+ (Transformation|GetActorLocation) (* _returnvalue (+ (Components|Capsule|GetScaledCapsuleRadius (Variables|Collision|GetCapsuleComponent)) 15.0))) "TraceTypeQuery1" true 0 "None"))
  (if _returnvalue_2
    (AddComponent|AddAudioComponent false)
    (Character|LaunchCharacter (Math|Vector|MakeVector (* (Math|Float|Sign(Float) (- (.x (Transformation|GetActorLocation)) (.x (.Location (Collision|BreakHitResult _outhit))))) 4e+02) 0.0 (Variables|/Script/Engine.CharacterMovementComponent|GetJumpZVelocity (Variables|Character|GetCharacterMovement))) false false)))

(event Custom|Damage
  (params (damageAmt :type Float%20%28single-precision%29))
  (bind _returnvalue (Transformation|GetActorRotation))
  (bind _returnvalue_2 (Math|Rotator|GetRotationXVector _returnvalue))
  ;[1 1 1] Damage
  (if (Variables|Default|GetcanBeHurt)
    (Variables|Default|SetcanBeHurt false)
    (bind _output_get (Variables|Default|SetHealth (- (Variables|Default|GetHealth) damageAmt)))
    (if (<= _output_get 0.0)
      (Variables|Default|SetisDead true)
      (Variables|Default|SetLives (- (Variables|Default|GetLives) 1))
      (if (> (Variables|Default|GetLives) 0)
        (Utilities|FlowControl|Delay 0.5)
        (Utilities|FlowControl|Sequence
          (:then_0
            (Variables|Default|SetisDead false))
          (:then_1
            (Actor|DestroyActor)))
        (else
          (Utilities|FlowControl|Delay 0.5)
          (Game|OpenLevel(byName) "GameOver_Lose")))
      (else
        (CallFunction|UpdateAnimation)
        (Character|LaunchCharacter (* (Math|Vector|RotateVector _returnvalue_2 (Math|Rotator|SelectRotator "-60.000000, 0, 0" "60.000000, 0, 0" (> (.X (Math|Vector|BreakVector _returnvalue_2)) 0.0))) -5e+02) true true)
        (CallFunction|UpdateAnimation)
        (Utilities|FlowControl|Delay 1.0)
        (Variables|Default|SetcanBeHurt true)))))

(event Custom|Spawn%20Player
  ;[1 1 1] Spawn Player
  (bind _asmy_game_instance (Utilities|Casting|CastToMyGameInstance (Game|GetGameInstance)))
  (if (Utilities|Name|Equal(Name) (Variables|/Game/Blueprints/MyGameInstance.MyGameInstance_C|GetgameLevel _asmy_game_instance) "GameLevel")
    (Transformation|SetActorLocation (Math|Vector|MakeVector (.x (Variables|/Game/Blueprints/MyGameInstance.MyGameInstance_C|GetSpawnLocation _asmy_game_instance)) 0.0 (+ (.z (Variables|/Game/Blueprints/MyGameInstance.MyGameInstance_C|GetSpawnLocation _asmy_game_instance)) 25.0)) false false)
    (Variables|Default|SetHealth (Variables|/Game/Blueprints/MyGameInstance.MyGameInstance_C|GetHealth _asmy_game_instance))))

(event EventBeginPlay
  ;[1 1 1] Init Plaayer
  (CallFunction|SpawnPlayer))

(event EventDestroyed
  ;[1 1 1] Respawns the Actor at spawn Location
  (bind _returnvalue (Game|SpawnActorfromClass "PlayerBP_C" (Variables|Default|GetTransformStartPoint) "Undefined" 0 0))
  (bind _output_get (Variables|Default|SetPlayer _returnvalue))
  (Pawn|Possess (Game|GetPlayerController 0) _output_get))

(event Input|ActionEvents|InputActionJump
  (params (Key :type Key%20Structure :default "AnyKey"))
  ;[1 1 1] Jumping
  (:Pressed
    (if (Variables|Default|GetisFalling)
      _
      (else
        (AddComponent|AddAudioComponent false)))
    (Character|Jump)
    (if (AI|Components|NavMovement|IsFalling (Variables|Character|GetCharacterMovement))
      (CallFunction|WallJump)))
  (:Released
    (Character|StopJumping)))

(event Input|ActionEvents|InputActionFiring
  (params (Key :type Key%20Structure :default "AnyKey"))
  ;[1 1 1] Firing
  (:Pressed
    (if (not (Variables|Default|GetisFalling))
      (if (> (Variables|Default|GetAmmoCnt) 0.0)
        (Audio|PlaySound2D "/Game/Sound/FX/Snd_Cue/Shoot_snd.Shoot_snd")
        (Variables|Default|SetAmmoCnt (- (Variables|Default|GetAmmoCnt) 1.0))
        (if (Variables|Default|GetisMoving)
          (Variables|Default|SetisFireMovement true)
          (Utilities|FlowControl|Delay 0.1)
          (Game|SpawnActorfromClass "/Game/Blueprints/Player/ProjectileBP.ProjectileBP_C" (Transformation|GetWorldTransform (Variables|Default|GetProjectileArrow)) "AlwaysSpawn" 0 0)
          (else
            (Variables|Default|SetisFiring true)
            (Utilities|FlowControl|Delay 0.1)
            (Game|SpawnActorfromClass "/Game/Blueprints/Player/ProjectileBP.ProjectileBP_C" (Transformation|GetWorldTransform (Variables|Default|GetProjectileArrow)) "AlwaysSpawn" 0 0)
            (Components|Movement|StopMovementImmediately (Variables|Character|GetCharacterMovement))))
        (CallFunction|UpdateAnimation :!label _label))))
  (:Released
    (Utilities|FlowControl|RetriggerableDelay 0.25)
    (Utilities|FlowControl|Sequence
      (:then_0
        (Variables|Default|SetisFiring false)
        (goto _label))
      (:then_1
        (Variables|Default|SetisFireMovement false)
        (goto _label)))))

(event Input|ActionEvents|InputActionDoor
  (params (Key :type Key%20Structure :default "AnyKey"))
  (bind _levelselected (Variables|Default|GetLevelSelected))
  ;[1 1 1] Enter Door
  (:Pressed
    (if (Variables|Default|GetisDoor)
      (bind _asmy_game_instance (Utilities|Casting|CastToMyGameInstance (Game|GetGameInstance)))
      (Variables|/Game/Blueprints/MyGameInstance.MyGameInstance_C|SetSpawnLocation _asmy_game_instance (Variables|/Game/Blueprints/MyGameInstance.MyGameInstance_C|GetSpawnLocation _asmy_game_instance))
      (Variables|/Game/Blueprints/MyGameInstance.MyGameInstance_C|SetHealth _asmy_game_instance (Variables|Default|GetMaxHealth))
      (Variables|/Game/Blueprints/MyGameInstance.MyGameInstance_C|SetGameStatus _asmy_game_instance true)
      (Variables|/Game/Blueprints/MyGameInstance.MyGameInstance_C|SetgameLevel _asmy_game_instance _levelselected)
      (Game|OpenLevel(byName) _levelselected))))

(event Input|AxisEvents|InputAxisMoveRight
  (params (AxisValue :type Float%20%28single-precision%29))
  ;[1 1 1] Movement
  (Utilities|FlowControl|Sequence
    (:then_0
      (if (not (Variables|Default|GetisFiring))
        (Pawn|Input|AddMovementInput "1.000000, 0, 0" AxisValue false :!label _label)
        (CallFunction|UpdateAnimation)
        (Math|Float|CompareFloat AxisValue 0.0
          (:>
            (Pawn|SetControlRotation (Pawn|GetController) (Math|Rotator|MakeRotator 0.0 0.0 0.0)))
          (:<
            (Pawn|SetControlRotation (Pawn|GetController) (Math|Rotator|MakeRotator 0.0 0.0 1.8e+02))))))
    (:then_1
      (if (Variables|Default|GetisFireMovement)
        (goto _label)))))

(event Input|KeyboardEvents|D
  (params (Key :type Key%20Structure :default "AnyKey"))
  (:Pressed
    (if (Variables|Default|GetisFalling)
      (Audio|Components|Audio|Stop (stale _returnvalue) :!label _label)
      (else
        (bind _returnvalue (AddComponent|AddAudioComponent false)))))
  (:Released
    (goto _label)))

(event Input|KeyboardEvents|A
  (params (Key :type Key%20Structure :default "AnyKey"))
  (:Pressed
    (if (Variables|Default|GetisFalling)
      (Audio|Components|Audio|Stop (stale _returnvalue) :!label _label)
      (else
        (bind _returnvalue (AddComponent|AddAudioComponent false)))))
  (:Released
    (goto _label)))

(fn ConstructionScript
  (Variables|Default|SetTransformStartPoint (Transformation|GetActorTransform)))

(fn AnimationStateMachine
  (params (isMoving :type Boolean) (isFalling :type Boolean) (Firing :type Boolean) (Hurt :type Boolean) (Death :type Boolean) (FireMovement :type Boolean))
  (LocalVariables|SetisMovingLocal isMoving)
  (LocalVariables|SetisFallingLocal isFalling)
  (LocalVariables|SetifFiringLocal Firing)
  (LocalVariables|SetisHurtLocal Hurt)
  (LocalVariables|SetisDeadLocal Death)
  (LocalVariables|SetisFireMovementLocal FireMovement)
  (if (LocalVariables|GetisFallingLocal)
    (LocalVariables|SetAnimationStates "NewEnumerator2")
    (elif (LocalVariables|GetifFiringLocal)
      (LocalVariables|SetAnimationStates "NewEnumerator3")
      (elif (LocalVariables|GetisHurtLocal)
        (LocalVariables|SetAnimationStates "NewEnumerator4")
        (elif (LocalVariables|GetisDeadLocal)
          (LocalVariables|SetAnimationStates "NewEnumerator5")
          (elif (LocalVariables|GetisFireMovementLocal)
            (LocalVariables|SetAnimationStates "NewEnumerator6")
            (elif (LocalVariables|GetisMovingLocal)
              (LocalVariables|SetAnimationStates "NewEnumerator1")
              (else
                (LocalVariables|SetAnimationStates "NewEnumerator0"))))))))
  (return (Utilities|Select :Index (LocalVariables|GetAnimationStates) :NewEnumerator0 (Variables|Animations|GetIdle%20Flipbook) :NewEnumerator1 (Variables|Animations|GetWalk%20Flipbook) :NewEnumerator2 (Variables|Animations|GetJump%20Flipbook) :NewEnumerator3 (Variables|Animations|GetFiring%20Flipbook) :NewEnumerator4 (Variables|Animations|GetHurt%20Flipbook) :NewEnumerator5 (Variables|Animations|GetDead%20Flipbook) :NewEnumerator6 (Variables|Animations|GetWalk%20Flipbook))))