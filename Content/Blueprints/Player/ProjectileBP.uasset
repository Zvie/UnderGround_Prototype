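; Player projectile Blueprint that damages zombies and the boss enemy on overlap.
; On ActorBeginOverlap, a sequence tries casts to the male zombie, female zombie and boss Blueprints in turn.
; A successful cast calls that enemy's DamageEnemy with DmgAmt, then spawns the ShotEffect emitter at the projectile's location and destroys it.
; Overlaps with any other actor are ignored, so the projectile is not destroyed by them.
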(event Collision|EventActorBeginOverlap
  (params (OtherActor :type Actor%20Object%20Reference))
  (bind _dmgamt (Variables|Default|GetdmgAmt))
  (Utilities|FlowControl|Sequence
    (:then_0
      (bind _asmale_zombie_bp (Utilities|Casting|CastToMale_Zombie_BP OtherActor))
      (Default|DamageEnemy _asmale_zombie_bp _dmgamt))
    (:then_1
      (bind _asfemale_zombie_bp (Utilities|Casting|CastToFemale_Zombie_BP OtherActor))
      (Default|DamageEnemy _asfemale_zombie_bp _dmgamt))
    (:then_2
      (bind _asboss_enemy_bp (Utilities|Casting|CastToBoss_enemy_BP OtherActor))
      (Default|DamageEnemy _asboss_enemy_bp _dmgamt)))
  (Effects|SpawnEmitteratLocation "/Game/Particles/shotEffect.shotEffect" (Transformation|GetActorLocation))
  (Actor|DestroyActor))

(fn ConstructionScript)