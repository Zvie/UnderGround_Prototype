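; Moving platform that shuttles a ledge sprite between StartPoint and EndPoint on a timeline, pausing before each reversal.
; A looping timer sphere-traces just below the ledge and plays the timeline forward again if the player is there during a reverse move.
; MovementRate sets both timeline speed and trace interval.
; With TestEndPoint on, the construction script previews the end position and zeroes the actor's Y.
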(event Custom|LookForObstruction
  (bind _movingledgesprite (Variables|Default|GetMovingLedgeSprite))
  (bind _returnvalue (Transformation|GetWorldLocation _movingledgesprite))
  ;[1 1 1] Look for Obstruction
  (bind _outhit (Collision|SphereTraceForObjects (- _returnvalue "0, 0,100.000000") (- _returnvalue "0, 0,101.000000") (/ (.SphereRadius (Collision|GetComponentBounds _movingledgesprite)) 2.0) (Utilities|Array|MakeArray "ObjectTypeQuery3") false 0 "None"))
  (Utilities|Casting|CastToPlayerBP (.hitactor _outhit))
  (if (Class|TimelineComponent|IsReversing)
    (CallFunction|ElevatorObstructed)))

(event Custom|ElevatorObstructed
  ;[1 1 1] Platform Movement
  (bind (_direction _newtrack_0) (Timeline|ElevatorTimeline Play)
    (:Update
      (Transformation|SetRelativeLocation (Variables|Default|GetMovingLedgeSprite) (Math|Vector|Lerp(Vector) (Variables|Default|GetStartPoint) (Variables|Default|GetEndPoint) _newtrack_0) false false))
    (:Finished
      (Utilities|FlowControl|Delay (Variables|Default|GetWaitTime))
      (switch Utilities|FlowControl|Switch|SwitchonETimelineDirection _direction
        (:Forward
          (Timeline|ElevatorTimeline ReverseFromEnd))
        (:Backward
          (Timeline|ElevatorTimeline PlayFromStart))))))

(event EventBeginPlay
  (bind _movementrate (Variables|Default|GetMovementRate))
  (bind _returnvalue (/ 1.0 _movementrate))
  ;[1 1 1] start Platform
  (Components|Timeline|SetPlayRate (Variables|Default|GetElevatorTimeline) _returnvalue)
  (Utilities|Time|SetTimerbyFunctionName 0 "LookForObstruction" _returnvalue true))

(fn ConstructionScript
  (bind _returnvalue (Transformation|GetActorLocation))
  (bind (_x _y _z) (Math|Vector|BreakVector _returnvalue))
  (if (Variables|Default|GetTestEndPoint)
    (Transformation|SetRelativeLocation (Variables|Default|GetMovingLedgeSprite) (Variables|Default|GetEndPoint) false false)
    (Transformation|SetActorLocation (Math|Vector|MakeVector _x 0.0 _z) false false)))